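; Interactable button Blueprint that animates a cube being pressed in and back out when the player uses Interact nearby.
; A Box overlap with ThirdPersonCharacter opens and closes a Gate that filters the Interact input.
; The ButtonIn timeline, followed by a reversed ButtonOut timeline, lerps the Cube's relative transform between the Box's initial relative transform and identity.
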(event `InputAction|Interact`
  (params (Key :type "Key Structure"))
  (:`Pressed`
    (`/Engine/EditorBlueprintResources/StandardMacros.Gate` true :!label _label
      (:`Exit`
        (bind (_direction _button_in) (`Timeline|Button In` :!via `PlayFromStart`)
          (:`Update`
            (`SceneComponent.K2_SetRelativeTransform` (`self.Cube`) (`KismetMathLibrary.TLerp` (`self.Out Position`) (`self.In Position`) _button_in) false false))
          (:`Finished`
            (bind (_direction_2 _button_in_2) (`Timeline|Button Out` :!via `ReverseFromEnd`)
              (:`Update`
                (`SceneComponent.K2_SetRelativeTransform` (`self.Cube`) (`KismetMathLibrary.TLerp` (`self.Out Position`) (`self.In Position`) _button_in_2) false false)))))))))

(event `self.ReceiveBeginPlay`
  (bind (_returnvalue_location _returnvalue_rotation _returnvalue_scale) (`KismetMathLibrary.BreakTransform` (`SceneComponent.GetRelativeTransform` (`self.Box`))))
  (set `self.Out Position` (`KismetMathLibrary.MakeTransform` _returnvalue_location _returnvalue_rotation _returnvalue_scale))
  (set `self.In Position` (`KismetMathLibrary.MakeTransform` (0.0 0.0 0.0))))

(event `self.Box.OnComponentBeginOverlap`
  (params (OverlappedComponent :type "PrimitiveComponent Object Reference") (OtherActor :type "Actor Object Reference") (OtherComp :type "PrimitiveComponent Object Reference") (OtherBodyIndex :type Integer) (bFromSweep :type Boolean) (SweepResult :type "HitResult Structure (by ref)"))
  (cast `/Game/ThirdPersonBP/Blueprints/ThirdPersonCharacter` OtherActor)
  (goto _label :!via `Open`))

(event `self.Box.OnComponentEndOverlap`
  (params (OverlappedComponent :type "PrimitiveComponent Object Reference") (OtherActor :type "Actor Object Reference") (OtherComp :type "PrimitiveComponent Object Reference") (OtherBodyIndex :type Integer))
  (cast `/Game/ThirdPersonBP/Blueprints/ThirdPersonCharacter` OtherActor)
  (goto _label :!via `Close`))

(fn `NewFunction_0`)

(fn `UserConstructionScript`)