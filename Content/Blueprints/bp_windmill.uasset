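; Windmill Blueprint that rotates its Axle component back and forth.
; Each Tick, Speed rises or falls by delta time until it passes the positive or negative SpeedCap, flipping the Increasing flag to reverse the ramp.
; Speed is applied directly as a per-frame world pitch rotation, so the spin rate is frame-rate dependent.
; The Box overlap event and construction script do nothing.
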(event `self.ReceiveTick`
  (params (DeltaSeconds :type "Float (single-precision)"))
  (bind _speed (`self.Speed`))
  (if (`self.increasing`)
    ;[1 1 1] Speed Increasing
    (bind _output_get (set `self.Speed` (+ _speed DeltaSeconds)))
    (if (> _output_get (`self.SpeedCap`))
      (set `self.increasing` false))
    (else
      ;[1 1 1] Speed Decreasing
      (bind _output_get_2 (set `self.Speed` (- _speed DeltaSeconds)))
      (if (< _output_get_2 (* (`self.SpeedCap`) -1.0))
        (set `self.increasing` true))))
  (`SceneComponent.K2_AddWorldRotation` (`self.Axle`) (`KismetMathLibrary.MakeRotator` 0.0 (`self.Speed`)) false false))

(event `self.Box.OnComponentBeginOverlap`
  (params (OverlappedComponent :type "PrimitiveComponent Object Reference") (OtherActor :type "Actor Object Reference") (OtherComp :type "PrimitiveComponent Object Reference") (OtherBodyIndex :type Integer) (bFromSweep :type Boolean) (SweepResult :type "HitResult Structure (by ref)")))

(fn `UserConstructionScript`)