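; Door actor that the player opens and closes by pressing its button with the Interact input.
; An interaction box enables input and opens a gate only while a ThirdPersonCharacter overlaps it.
; Interact runs the ButtonPressAnim timeline to move the button, then a FlipFlop plays or reverses DoorTimeline to swing the door's yaw between closed and open angles.
; The construction script places the button from ButtonTransform.
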(event `InputAction|Interact`
  (params (Key :type "Key Structure"))
  ;[1 1 1] Hit E
  (:`Pressed`
    (`/Engine/EditorBlueprintResources/StandardMacros.Gate` true :!label _label
      (:`Exit`
        ;[1 1 1] Push Button
        (bind (_direction _newtrack_0) (`Timeline|Timeline_0` :!via `PlayFromStart`)
          (:`Update`
            (`SceneComponent.K2_SetRelativeLocation` (`self.Button`) (`KismetMathLibrary.VLerp` (`self.Button Out`) (`self.Button In`) _newtrack_0) false false))
          (:`Finished`
            (`KismetSystemLibrary.PrintString` "Hello")
            ;[1 1 1] Door Open and Close
            (`/Engine/EditorBlueprintResources/StandardMacros.FlipFlop`
              (:`A`
                (bind (_direction_2 _doortrack) (`Timeline|DoorTimeline` :!label _label_2)
                  (:`Update`
                    (`SceneComponent.K2_SetRelativeRotation` (`self.Door`) (`KismetMathLibrary.MakeRotator` 0.0 0.0 (`KismetMathLibrary.Lerp` (`self.Door Close Angle`) (`self.Door Open Angle`) _doortrack)) false false))))
              (:`B`
                (goto _label_2 :!via `Reverse`)))))))))

(event `self.InteractionBox.OnComponentBeginOverlap`
  (params (OverlappedComponent :type "PrimitiveComponent Object Reference") (OtherActor :type "Actor Object Reference") (OtherComp :type "PrimitiveComponent Object Reference") (OtherBodyIndex :type Integer) (bFromSweep :type Boolean) (SweepResult :type "HitResult Structure (by ref)"))
  ;[1 1 1] Hit E
  (cast `/Game/ThirdPersonBP/Blueprints/ThirdPersonCharacter` OtherActor)
  (`self.EnableInput` (`GameplayStatics.GetPlayerController` 0))
  (goto _label :!via `Open`))

(event `self.InteractionBox.OnComponentEndOverlap`
  (params (OverlappedComponent :type "PrimitiveComponent Object Reference") (OtherActor :type "Actor Object Reference") (OtherComp :type "PrimitiveComponent Object Reference") (OtherBodyIndex :type Integer))
  ;[1 1 1] Hit E
  (cast `/Game/ThirdPersonBP/Blueprints/ThirdPersonCharacter` OtherActor)
  (`self.DisableInput` (`GameplayStatics.GetPlayerController` 0))
  (goto _label :!via `Close`))

(fn `UserConstructionScript`
  (`SceneComponent.K2_SetRelativeTransform` (`self.Button`) (`self.Button Transform`) false false))